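; Pickup actor that grants the player HP, ammo or a damage boost according to its CollectibleType.
; On overlap it plays a sound for any actor, then applies the reward only to Player-tagged BP_ThirdPersonCharacters and hides itself.
; SetVisibility toggles spawned state, visibility, collision and tick for reuse without destruction, rerolling type and sphere material.
; RandomInteger(2) yields only HP or ammo, so that reroll never selects damage boost.
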(event `self.ReceiveActorBeginOverlap`
  (params (OtherActor :type "Actor Object Reference"))
  (bind _collectibletype (`self.CollectibleType`))
  (`GameplayStatics.PlaySound2D` "/Game/SFX/PickupSFX.PickupSFX" 1.0 1.0 0.0 null null)
  (if (== (`|GetArrayItem` (`Actor.Tags` OtherActor)) "Player")
    (bind _asbp_third_person_character (cast `/Game/ThirdPerson/Blueprints/BP_ThirdPersonCharacter` OtherActor))
    (if (== _collectibletype 0)
      (`/Game/ThirdPerson/Blueprints/BP_ThirdPersonCharacter.AddHP` _asbp_third_person_character)
      (elif (== _collectibletype 1)
        (`/Game/ThirdPerson/Blueprints/BP_ThirdPersonCharacter.AddAmmo` _asbp_third_person_character)
        (else
          (`/Game/ThirdPerson/Blueprints/BP_ThirdPersonCharacter.AddDamageBoost` _asbp_third_person_character))))
    (`self.SetVisibility` false)))

(fn `SetVisibility`
  (params (IsVisible :type Boolean))
  (bind _sphere (`self.Sphere`))
  (set `self.IsSpawned` IsVisible)
  (`self.SetActorHiddenInGame` (not IsVisible))
  (`self.SetActorEnableCollision` IsVisible)
  (`self.SetActorTickEnabled` IsVisible)
  (bind _output_get (set `self.CollectibleType` (`KismetMathLibrary.RandomInteger` 2)))
  (if (== _output_get 0)
    (`PrimitiveComponent.SetMaterial` _sphere 0 (`self.HpMaterial`))
    (elif (== _output_get 1)
      (`PrimitiveComponent.SetMaterial` _sphere 0 (`self.AmmoMaterial`))
      (else
        (`PrimitiveComponent.SetMaterial` _sphere 0 (`self.DmgMaterial`))))))

(fn `UserConstructionScript`)